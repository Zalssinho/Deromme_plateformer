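; BP_Player is the player Blueprint that creates the main HUD and handles collecting, interacting and triggering elevating platforms.
; Overlaps pass collectible components to its collect component and refresh the blue score on the HUD.
; Overlapping a BPI_Interract actor arms the interact input, which sends ActiveMessage until that actor's overlap ends.
; Hits send ElevateMessage to BPI_Elevate actors, so components and interfaces avoid casting.
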(event `self.ReceiveBeginPlay`
  (`parent.ReceiveBeginPlay`)
  ;[1 1 1] Widget HUD point score
  (bind _returnvalue (`|CreateWidget` "/Game/Game/BluePrint/Widget/BPW_MainHUD.BPW_MainHUD_C"))
  (`UserWidget.AddToViewport` _returnvalue 0)
  (set `self.HUD` _returnvalue))

(event `self.ReceiveActorBeginOverlap`
  (params (OtherActor :type "Actor Object Reference"))
  ;[1 1 1] Fonction Collect Object
  (`|ExecutionSequence`
    (:`then_0`
      (`self.CollectingObject` OtherActor))
    (:`then_1`
      ;[1 1 1] Fonction Interract
      (`self.Interract` OtherActor))))

(event `self.ReceiveHit`
  (params (MyComp :type "PrimitiveComponent Object Reference") (Other :type "Actor Object Reference") (OtherComp :type "PrimitiveComponent Object Reference") (bSelfMoved :type Boolean) (HitLocation :type "Vector Structure") (HitNormal :type "Vector Structure") (NormalImpulse :type "Vector Structure") (Hit :type "HitResult Structure (by ref)"))
  ;[1 1 1] Activation de la plateforme
  (`self.UpdatePlateforme` Other))

(event `self.ReceiveActorEndOverlap`
  (params (OtherActor :type "Actor Object Reference"))
  ;[1 1 1] Faire en sorte que lorque l'on sorte de la box collision on ne peux plus appuyer sur E
  (if (== OtherActor (`self.InteractableActor`))
    (set `self.CanActivate` false)))

(event `EnhancedInput|/Game/ThirdPerson/Input/Actions/IA_Interract`
  (params (ActionValue :type Boolean) (ElapsedSeconds :type "Float (double-precision)") (TriggeredSeconds :type "Float (double-precision)") (InputAction :type "InputAction Object Reference" :default "/Game/ThirdPerson/Input/Actions/IA_Interract.IA_Interract"))
  ;[1 1 1] E interraction
  (:`Started`
    (if (`self.CanActivate`)
      (message `/Game/Game/BluePrint/BPI/BPI_Interract.Active` (`self.InteractableActor`)))))

(fn `CollectingObject`
  (params (`Other Actor` :type "Actor Object Reference"))
  (bind _returnvalue (`self.GetComponentByClass` `Other Actor` "/Game/Game/BluePrint/Component/BPC_CollectibleComponent.BPC_CollectibleComponent_C"))
  (`/Engine/EditorBlueprintResources/StandardMacros.IsValid` _returnvalue
    (:`Is Valid`
      (`/Game/Game/BluePrint/Component/BPC_CollectComponent.Collect` (`self.BPC_CollectComponent`) _returnvalue)
      (`/Game/Game/BluePrint/Widget/BPW_MainHUD.UpdateScoreBlue` (`self.HUD`)))))

(fn `Interract`
  (params (`Other Actor` :type "Actor Object Reference"))
  (if (`KismetSystemLibrary.DoesImplementInterface` `Other Actor` "/Game/Game/BluePrint/BPI/BPI_Interract.BPI_Interract_C")
    (set `self.InteractableActor` `Other Actor`)
    (set `self.CanActivate` true)))

(fn `UpdatePlateforme`
  (params (`Other Actor` :type "Actor Object Reference"))
  (if (`KismetSystemLibrary.DoesImplementInterface` `Other Actor` "/Game/Game/BluePrint/BPI/BPI_Elevate.BPI_Elevate_C")
    (message `/Game/Game/BluePrint/BPI/BPI_Elevate.Elevate` `Other Actor`)))

(fn `UserConstructionScript`
  (`parent.UserConstructionScript`))