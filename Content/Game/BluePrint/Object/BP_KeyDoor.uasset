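; BP_KeyDoor is a door that swings open and closed on activation, gated by the key value in the game instance.
; It caches BP_GameInstance on BeginPlay, and Active proceeds only when its Key equals 2.
; A FlipFlop alternates playing a timeline from start and reversing it, with the squared timeline value driving the Door component's relative yaw for an eased quarter-turn swing.
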(event `self.ReceiveBeginPlay`
  (bind _asbp_game_instance (cast `/Game/Game/BluePrint/BP_GameInstance` (`GameplayStatics.GetGameInstance`)))
  (set `self.As BP Game Instance` _asbp_game_instance))

(event `/Game/Game/BluePrint/BPI/BPI_Interract.Active`
  (if (== (`/Game/Game/BluePrint/BP_GameInstance.Key` (`self.As BP Game Instance`)) 2)
    (`/Engine/EditorBlueprintResources/StandardMacros.FlipFlop`
      (:`A`
        (bind (_direction _doorfloat) (`Timeline|Timeline` :!via `PlayFromStart` :!label _label)
          (:`Update`
            (`SceneComponent.K2_SetRelativeRotation` (`self.Door`) (`KismetMathLibrary.MakeRotator` 0.0 0.0 (`KismetMathLibrary.Lerp` 0.0 -90.0 (`KismetMathLibrary.MultiplyMultiply_FloatFloat` _doorfloat 2.0))) false false))))
      (:`B`
        (goto _label :!via `Reverse`)))))

(fn `UserConstructionScript`)