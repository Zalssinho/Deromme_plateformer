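; BP_Light is a light actor whose on/off state comes from light states held in BP_GameInstance.
; On BeginPlay it caches the game instance, binds UpdateLight to its OnLightToggle event and syncs once.
; UpdateLight looks up the state for the light's Numbre and applies it to the PointLight's visibility.
; The Active event is empty, and a FlipFlop visibility toggle is left disconnected.
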(event `self.ReceiveBeginPlay`
  ;[1 1 1] Récupérer le gameinstance
  (bind _asbp_game_instance (cast `/Game/Game/BluePrint/BP_GameInstance` (`GameplayStatics.GetGameInstance`)))
  (bind _output_get (set `self.As BP Game Instance` _asbp_game_instance))
  (add `/Game/Game/BluePrint/BP_GameInstance.OnLightToggle` _output_get (delegate `UpdateLight`))
  (`self.UpdateLight`))

(event `UpdateLight`
  ;[1 1 1] Update les lights grace à l'évènement
  (bind _lightstaes (`/Game/Game/BluePrint/BP_GameInstance.GetLightStatesByNumber` (`self.As BP Game Instance`) (`self.Numbre`)))
  (`SceneComponent.SetVisibility` (`self.PointLight`) _lightstaes false))

(event `/Game/Game/BluePrint/BPI/BPI_Interract.Active`
  ;[1 1 1] Lumière On/Off
)

(fn `UserConstructionScript`)