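; BP_Door is a door actor that swings open or closed according to a door state held in BP_GameInstance.
; On BeginPlay it binds UpdateDoorState to the GameInstance's light-toggle event and opens if the state is already true.
; UpdateDoorState reads that state and plays or reverses a Timeline, whose squared alpha drives a yaw lerp on the Door component.
; A second, unconnected OpenDoorTimeline duplicates that rotation.
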(event `self.ReceiveBeginPlay`
  ;[1 1 1] Communication au GameInstance
  (bind _asbp_game_instance (cast `/Game/Game/BluePrint/BP_GameInstance` (`GameplayStatics.GetGameInstance`)))
  (bind _output_get (set `self.As BP Game Instance` _asbp_game_instance))
  (add `/Game/Game/BluePrint/BP_GameInstance.OnLightToggle` _output_get (delegate `UpdateDoorState`))
  (bind _doorstate (`/Game/Game/BluePrint/BP_GameInstance.GetDoorState` (`self.As BP Game Instance`)))
  (if _doorstate
    (`self.UpdateDoorState`)))

(event `UpdateDoorState`
  (bind _doorstate (`/Game/Game/BluePrint/BP_GameInstance.GetDoorState` (`self.As BP Game Instance`)))
  (if _doorstate
    (bind (_direction _doorfloat) (`Timeline|Timeline` :!via `PlayFromStart` :!label _label)
      (:`Update`
        (`SceneComponent.K2_SetRelativeRotation` (`self.Door`) (`KismetMathLibrary.MakeRotator` 0.0 0.0 (`KismetMathLibrary.Lerp` 0.0 -90.0 (`KismetMathLibrary.MultiplyMultiply_FloatFloat` _doorfloat 2.0))) false false)))
    (else
      (goto _label :!via `Reverse`))))

(event `/Game/Game/BluePrint/BPI/BPI_Interract.Active`
  ;[1 1 1] Ouverture et fermeture de la porte + Timeline
)

(fn `UserConstructionScript`)