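; BPC_CollectComponent is an actor component that handles picking up blue and yellow mana collectibles.
; On BeginPlay it casts and caches the BP_GameInstance, which holds both mana scores.
; Collect adds the collectible's Value to the blue or yellow score based on IsBlue, then calls DestroyBPCollectible on it.
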(event `self.ReceiveBeginPlay`
  ;[1 1 1] Communication entre le BPC_CollectComponent et Game Instance
  (bind _asbp_game_instance (cast `/Game/Game/BluePrint/BP_GameInstance` (`GameplayStatics.GetGameInstance`)))
  (set `self.BP_GameInstance` _asbp_game_instance))

(fn `Collect`
  (params (Mana :type "/Game/Game/BluePrint/Component/BPC_CollectibleComponentMana Object Reference"))
  (bind _bp_gameinstance (`self.BP_GameInstance`))
  (bind _value (`/Game/Game/BluePrint/Component/BPC_CollectibleComponentMana.Value` Mana))
  ;[1 1 1] Augmentation du Score en utilisant la game instance et BPC_Collectibles
  (if (`/Game/Game/BluePrint/Component/BPC_CollectibleComponentMana.IsBlue` Mana)
    (set `/Game/Game/BluePrint/BP_GameInstance.ScoreManaBlue` (+ _value (`/Game/Game/BluePrint/BP_GameInstance.ScoreManaBlue` _bp_gameinstance)) _bp_gameinstance)
    (else
      (set `/Game/Game/BluePrint/BP_GameInstance.ScoreManeYellow` (+ _value (`/Game/Game/BluePrint/BP_GameInstance.ScoreManeYellow` _bp_gameinstance)) _bp_gameinstance)))
  (`/Game/Game/BluePrint/Component/BPC_CollectibleComponentMana.DestroyBPCollectible` Mana))