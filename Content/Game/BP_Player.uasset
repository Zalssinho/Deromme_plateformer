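; BP_Player is the player actor that creates the main HUD and picks up collectibles it overlaps.
; On BeginPlay it adds a BPW_MainHUD widget to the viewport and keeps a reference to it.
; Each overlap passes any BPC_CollectibleComponent on the other actor to BPCCollectComponent, refreshes the HUD score, then calls ActiveMessage on that actor whether or not it was collectible.
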(event `self.ReceiveBeginPlay`
  (`parent.ReceiveBeginPlay`)
  (bind _returnvalue (`|CreateWidget` "/Game/Game/BPW_MainHUD.BPW_MainHUD_C"))
  (`UserWidget.AddToViewport` _returnvalue 0)
  (set `self.HUD` _returnvalue))

(event `self.ReceiveActorBeginOverlap`
  (params (OtherActor :type "Actor Object Reference"))
  (`|ExecutionSequence`
    (:`then_0`
      (`self.CollectingObject` OtherActor))
    (:`then_1`
      (message `/Game/Game/BPI_Interract.Active` OtherActor))))

(event `EnhancedInput|/Game/ThirdPerson/Input/Actions/IA_Interract`
  (params (ActionValue :type Boolean) (ElapsedSeconds :type "Float (double-precision)") (TriggeredSeconds :type "Float (double-precision)") (InputAction :type "InputAction Object Reference" :default "/Game/ThirdPerson/Input/Actions/IA_Interract.IA_Interract")))

(fn `CollectingObject`
  (params (`Other Actor` :type "Actor Object Reference"))
  (bind _returnvalue (`self.GetComponentByClass` `Other Actor` "/Game/Game/BPC_CollectibleComponent.BPC_CollectibleComponent_C"))
  (`/Engine/EditorBlueprintResources/StandardMacros.IsValid` _returnvalue
    (:`Is Valid`
      (`/Game/Game/BPC_CollectComponent.Collect` (`self.BPC_CollectComponent`) _returnvalue)
      (`/Game/Game/BPW_MainHUD.UpdateScore` (`self.HUD`)))))

(fn `UserConstructionScript`
  (`parent.UserConstructionScript`))